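; Damage platform whose spikes animate and hurt the BP_ThirdPersonCharacter that steps on it.
; Box overlap starts a two-second, non-looping timer, and leaving the box before it fires cancels it.
; When the timer fires, a timeline moves the spikes along Z and its event track applies damage to the stored character, with no re-check that they are still overlapping.
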(event `self.Box.OnComponentBeginOverlap`
  (params (OverlappedComponent :type "PrimitiveComponent Object Reference") (OtherActor :type "Actor Object Reference") (OtherComp :type "PrimitiveComponent Object Reference") (OtherBodyIndex :type Integer) (bFromSweep :type Boolean) (SweepResult :type "HitResult Structure (by ref)"))
  (bind _asbp_third_person_character (cast `/Game/ThirdPerson/OlafThings/Blueprints/BP_ThirdPersonCharacter` OtherActor))
  (bind _returnvalue (`KismetSystemLibrary.K2_SetTimerDelegate` (delegate `AplicarDaño`) 2.0))
  (set `self.TimerPlataforma` _returnvalue))

(event `AplicarDaño`
  (bind (_direction _posicion_z) (`Timeline|Animacion pinchos` :!via `PlayFromStart`)
    (:`Update`
      (`SceneComponent.K2_SetRelativeLocation` (`self.Pinchos`) (`KismetMathLibrary.MakeVector` 0.0 0.0 _posicion_z) false false))
    (:`Hacer daño`
      (`GameplayStatics.ApplyDamage` (stale `self.Box.OnComponentBeginOverlap` _asbp_third_person_character) 1.0))))

(event `self.Box.OnComponentEndOverlap`
  (params (OverlappedComponent :type "PrimitiveComponent Object Reference") (OtherActor :type "Actor Object Reference") (OtherComp :type "PrimitiveComponent Object Reference") (OtherBodyIndex :type Integer))
  (cast `/Game/ThirdPerson/OlafThings/Blueprints/BP_ThirdPersonCharacter` OtherActor)
  (`KismetSystemLibrary.K2_ClearAndInvalidateTimerHandle` (`self.TimerPlataforma`)))

(fn `UserConstructionScript`)