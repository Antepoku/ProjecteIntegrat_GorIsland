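; BP_StartLevel is a trigger actor that plays a short camera cutaway to CameraPuerta, apparently a door camera, when its box is overlapped.
; A DoOnce gates timed view-target blends to that camera and back to the player character, then resets so the cutaway can replay.
; It also gathers all BP_Toogle_Platform actors, but the loop over them does nothing.
; The overlapping actor is not checked.
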(event `self.Box.OnComponentBeginOverlap`
  (params (OverlappedComponent :type "PrimitiveComponent Object Reference") (OtherActor :type "Actor Object Reference") (OtherComp :type "PrimitiveComponent Object Reference") (OtherBodyIndex :type Integer) (bFromSweep :type Boolean) (SweepResult :type "HitResult Structure (by ref)"))
  (bind _returnvalue (`GameplayStatics.GetPlayerController` 0))
  (`/Engine/EditorBlueprintResources/StandardMacros.DoOnce` false :!label _label
    (:`Completed`
      (bind _outactors (`GameplayStatics.GetAllActorsOfClass` "/Game/BluePrints_Hugo/BP_Toogle_Platform.BP_Toogle_Platform_C"))
      (for _ _outactors
        _)
      (`PlayerController.SetViewTargetWithBlend` _returnvalue (`self.CameraPuerta`) 1.5 "VTBlend_Linear" 0.0 true)
      (`KismetSystemLibrary.Delay` 1.5)
      (`KismetSystemLibrary.Delay` 1.0)
      (`PlayerController.SetViewTargetWithBlend` _returnvalue (`GameplayStatics.GetPlayerCharacter` 0) 0.6 "VTBlend_Linear" 0.0 true)
      (`KismetSystemLibrary.Delay` 0.6)
      (goto _label :!via `Reset`))))

(fn `UserConstructionScript`)