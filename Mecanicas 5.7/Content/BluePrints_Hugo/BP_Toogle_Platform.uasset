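; Toggleable platform actor that exists or vanishes in the level based on its IsActive flag.
; UpdateState shows the Cube mesh with query and physics collision when active, or hides it and disables collision when inactive.
; BeginPlay applies the initial state; nothing in this Blueprint changes IsActive afterwards.
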(event `self.ReceiveBeginPlay`
  (`self.UpdateState`))

(fn `UpdateState`
  (if (`self.IsActive`)
    (`SceneComponent.SetHiddenInGame` (`self.Cube`) false false)
    (`PrimitiveComponent.SetCollisionEnabled` (`self.Cube`) "QueryAndPhysics")
    (else
      (`SceneComponent.SetHiddenInGame` (`self.Cube`) true false)
      (`PrimitiveComponent.SetCollisionEnabled` (`self.Cube`) "NoCollision"))))

(fn `UserConstructionScript`)