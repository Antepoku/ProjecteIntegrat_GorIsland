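; BP_Plataforma_Temporal is a temporary platform that destroys itself shortly after any overlap with its Box trigger.
; BeginPlay gives the Cube a dynamic M_Light material instance with its M_Light scalar at zero.
; Overlap raises that scalar and plays the Opacity timeline, whose update writes a constant to the Opacity parameter rather than a curve value.
; A short Delay, started alongside the timeline, then destroys the actor.
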(event `self.ReceiveBeginPlay`
  (bind _returnvalue (`PrimitiveComponent.CreateDynamicMaterialInstance` (`self.Cube`) 0 "/Game/BluePrints_Hugo/Materiales_Hugo/M_Light.M_Light" "None"))
  (bind _output_get (set `self.Dynamic Material` _returnvalue))
  (`MaterialInstanceDynamic.SetScalarParameterValue` _output_get "M_Light" 0.0))

(event `self.Box.OnComponentBeginOverlap`
  (params (OverlappedComponent :type "PrimitiveComponent Object Reference") (OtherActor :type "Actor Object Reference") (OtherComp :type "PrimitiveComponent Object Reference") (OtherBodyIndex :type Integer) (bFromSweep :type Boolean) (SweepResult :type "HitResult Structure (by ref)"))
  (`MaterialInstanceDynamic.SetScalarParameterValue` (`self.Dynamic Material`) "M_Light" 10.0)
  (`|ExecutionSequence`
    (:`then_0`
      (`Timeline|Opacity`
        (:`Update`
          (`MaterialInstanceDynamic.SetScalarParameterValue` (`self.Dynamic Material`) "Opacity" 10.0))))
    (:`then_1`
      (`KismetSystemLibrary.Delay` 0.7)
      (`self.K2_DestroyActor`))))

(fn `UserConstructionScript`)