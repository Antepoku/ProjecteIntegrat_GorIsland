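; Toggleable platform actor (type A) that appears or disappears by switching its visibility and collision together.
; BeginPlay hides it if EstaEncendida is true and shows it otherwise, then inverts the flag.
; AlternarEstado shows and enables it when the flag is true, or hides and disables it when false, without changing the flag itself.
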(event `self.ReceiveBeginPlay`
  (if (`self.Esta encendida`)
    (`self.SetActorHiddenInGame` true)
    (`self.SetActorEnableCollision` false)
    (set `self.Esta encendida` false)
    (else
      (`self.SetActorHiddenInGame` false)
      (`self.SetActorEnableCollision` true)
      (set `self.Esta encendida` true))))

(event `Alternar Estado`
  (if (`self.Esta encendida`)
    (`self.SetActorHiddenInGame` false)
    (`self.SetActorEnableCollision` true)
    (else
      (`self.SetActorHiddenInGame` true)
      (`self.SetActorEnableCollision` false))))

(fn `UserConstructionScript`)