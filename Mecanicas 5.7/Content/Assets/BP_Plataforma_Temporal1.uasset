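; Temporary platform actor that lights up and destroys itself shortly after something overlaps its Box.
; BeginPlay stores the Cube's position and creates a dynamic palette material with the light off.
; Overlap turns on the light, plays an Opacity timeline that writes a constant Opacity value, and destroys the actor after a short delay.
; A Vibracion timeline for shaking the Cube along X is only ever stopped, never started by the graph.
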(event `self.ReceiveBeginPlay`
  (bind _cube (`self.Cube`))
  (bind _output_get (set `self.Posicion inicial` (`SceneComponent.RelativeLocation` _cube)))
  (bind _returnvalue (`PrimitiveComponent.CreateDynamicMaterialInstance` _cube 0 "/Game/Assets/Materials/MM_PaletteColor_Inst.MM_PaletteColor_Inst" "None"))
  (bind _output_get_2 (set `self.Dynamic Material` _returnvalue))
  (`MaterialInstanceDynamic.SetScalarParameterValue` _output_get_2 "M_Light" 0.0))

(event `self.Box.OnComponentBeginOverlap`
  (params (OverlappedComponent :type "PrimitiveComponent Object Reference") (OtherActor :type "Actor Object Reference") (OtherComp :type "PrimitiveComponent Object Reference") (OtherBodyIndex :type Integer) (bFromSweep :type Boolean) (SweepResult :type "HitResult Structure (by ref)"))
  (`TimelineComponent.Stop` (`self.Vibracion`))
  (`MaterialInstanceDynamic.SetScalarParameterValue` (`self.Dynamic Material`) "M_Light" 10.0)
  (`|ExecutionSequence`
    (:`then_0`
      (`Timeline|Opacity`
        (:`Update`
          (`MaterialInstanceDynamic.SetScalarParameterValue` (`self.Dynamic Material`) "Opacity" 10.0))))
    (:`then_1`
      (`KismetSystemLibrary.Delay` 0.7)
      (`self.K2_DestroyActor`))))

(fn `UserConstructionScript`)