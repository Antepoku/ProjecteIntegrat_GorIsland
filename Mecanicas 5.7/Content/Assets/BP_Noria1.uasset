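; BP_Noria1 is a rotating "noria" (Ferris-wheel style) actor with four cubes that keep a fixed orientation while the pivot turns.
; Each Tick, it adds local yaw to Pivote, scaled by VelocidadGiro and delta time for frame-rate-independent spin.
; It then resets the world rotation of all four cubes to zero, so they stay world-aligned like gondolas.
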(event `self.ReceiveTick`
  (params (DeltaSeconds :type "Float (single-precision)"))
  (`SceneComponent.K2_AddLocalRotation` (`self.Pivote`) (`KismetMathLibrary.MakeRotator` 0.0 0.0 (* DeltaSeconds (`self.Velocidad Giro`))) false false)
  (`SceneComponent.K2_SetWorldRotation` :`self` (`self.Cube1`))
  (`SceneComponent.K2_SetWorldRotation` :`self` (`self.Cube2`))
  (`SceneComponent.K2_SetWorldRotation` :`self` (`self.Cube3`))
  (`SceneComponent.K2_SetWorldRotation` :`self` (`self.Cube4`)))

(fn `UserConstructionScript`)